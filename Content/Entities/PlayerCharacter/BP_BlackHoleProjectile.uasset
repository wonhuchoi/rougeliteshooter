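; Black hole projectile fired by the player, which pulls physics objects with a radial force and swallows them.
; On spawn it ignores its instigator for movement and removes pawns from the radial force's affected object types.
; Any overlapped component that simulates physics gets its owning actor destroyed.
; A timer destroys the projectile itself after a few seconds.
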(event `self.ReceiveBeginPlay`
  (`KismetSystemLibrary.K2_SetTimerDelegate` (delegate `OnTimerElapsed`) 5.0)
  (`PrimitiveComponent.IgnoreActorWhenMoving` (`self.sphereComp`) (`self.GetInstigator`) true)
  (`RadialForceComponent.RemoveObjectTypeToAffect` (`self.RadialForce`) "ObjectTypeQuery3"))

(event `OnTimerElapsed`
  (`self.K2_DestroyActor`))

(event `self.sphereComp.OnComponentBeginOverlap`
  (params (OverlappedComponent :type "PrimitiveComponent Object Reference") (OtherActor :type "Actor Object Reference") (OtherComp :type "PrimitiveComponent Object Reference") (OtherBodyIndex :type Integer) (bFromSweep :type Boolean) (SweepResult :type "HitResult Structure (by ref)"))
  (if (`SceneComponent.IsSimulatingPhysics` OtherComp "None")
    (`self.K2_DestroyActor` OtherActor)))

(fn `UserConstructionScript`)